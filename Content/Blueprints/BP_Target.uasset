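; BP_Target is a shootable target actor for an aim trainer game.
; It starts hidden, with collision and tick disabled, and contains no logic to show itself.
; When a FirstPersonProjectile hits its Target component while visible, it hides and disables itself again, then tells GM_AimTrainer to spawn a new target, so it is reused rather than destroyed.
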(event OnComponentHit(Target)
  (params (HitComponent :type Primitive%20Component%20Object%20Reference) (OtherActor :type Actor%20Object%20Reference) (OtherComp :type Primitive%20Component%20Object%20Reference) (NormalImpulse :type Vector :default "0, 0, 0") (Hit :type Hit%20Result%20Structure%20%28by%20ref%29))
  (Utilities|Casting|CastToFirstPersonProjectile OtherActor)
  (bind _asgm_aim_trainer (Utilities|Casting|CastToGM_AimTrainer (Game|GetGameMode)))
  (if (not (Variables|Default|GetIsHidden?))
    (Variables|Default|SetIsHidden? true)
    (Rendering|SetActorHiddenInGame true)
    (Collision|SetActorEnableCollision false)
    (Actor|Tick|SetActorTickEnabled false)
    (Default|SpawnNewTarget _asgm_aim_trainer)))

(event EventBeginPlay
  (Variables|Default|SetIsHidden? true)
  (Rendering|SetActorHiddenInGame true)
  (Collision|SetActorEnableCollision false)
  (Actor|Tick|SetActorTickEnabled false))

(fn ConstructionScript)