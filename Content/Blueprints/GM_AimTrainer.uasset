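; Game mode for an aim trainer that reveals random pre-placed targets and runs a timed round.
; BeginPlay gathers all BP_Target actors, adds the UI, reveals the first target and starts a one-second countdown.
; SpawnNewTarget increments the hit score, including on that first call, then unhides a random existing target rather than spawning one.
; When time runs out, Endgame shows the score screen and switches to UI-only input.
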(event Custom|Spawn%20New%20Target
  (bind _result (Math|Integer|IncrementInt (Variables|Default|GetTargetHit))
    (:%20%20
      (Variables|Default|SetTargetHit _result)
      (Default|UpdateScore (Variables|Default|GetUIRef))
      (bind _result_2 (Math|Integer|DecrementInt (Utilities|Array|Length (Variables|Default|GetTargets)))
        (:%20%20
          (Variables|Default|SetNextTarget%20Index (Math|Random|RandomIntegerinRange 0 _result_2))
          (for (_array_element _array_index) (Variables|Default|GetTargets)
            (if (== _array_index (Variables|Default|GetNextTarget%20Index))
              ;[1 1 1] Chosen Target Is Visible
              (Rendering|SetActorHiddenInGame _array_element false)
              (Collision|SetActorEnableCollision _array_element true)
              (Actor|Tick|SetActorTickEnabled _array_element true)
              (Variables|/Game/Blueprints/BP_Target.BP_Target_C|SetIsHidden? _array_element false))))))))

(event Custom|DecrementCount
  (bind _time (Variables|Default|GetTime))
  (if (not (Variables|Default|GetIsgameOver?))
    (Math|Integer|DecrementInt _time
      (:%20%20
        (if (>= _time 0)
          (Default|UpdateCountdownText (Variables|Default|GetUIRef))
          (else
            (Variables|Default|SetIsgameOver? true)
            (CallFunction|Endgame (Variables|Default|GetTargetHit))))))))

(event EventBeginPlay
  (Input|SetInputModeGameOnly (Game|GetPlayerController 0))
  (bind _outactors (Actor|GetAllActorsOfClass "/Game/Blueprints/BP_Target.BP_Target_C"))
  (Variables|Default|SetTargets _outactors)
  (bind _returnvalue (UserInterface|CreateWidget "/Game/Blueprints/WBP_UI.WBP_UI_C"))
  (bind _output_get (Variables|Default|SetUIRef _returnvalue))
  (UserInterface|Viewport|AddtoViewport _output_get 0)
  (CallFunction|SpawnNewTarget)
  (Utilities|Time|SetTimerbyEvent (delegate Custom|DecrementCount) 1.0 true))

(fn ConstructionScript)

(fn Endgame
  (params (Score :type Integer))
  (bind _returnvalue (Game|GetPlayerController 0))
  (bind _returnvalue_2 (UserInterface|CreateWidget "/Game/Blueprints/WBP_EndScreen.WBP_EndScreen_C" 0 Score))
  (UserInterface|Viewport|AddtoViewport _returnvalue_2 0)
  (Input|SetInputModeUIOnly _returnvalue _returnvalue_2 "DoNotLock")
  (Input|SetIgnoreMoveInput _returnvalue true)
  (Variables|/Script/Engine.PlayerController|SetbShowMouseCursor _returnvalue true))